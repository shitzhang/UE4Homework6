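; BP_GrenadeProjectile is a grenade projectile that detonates in a small explosion.
; Its Explode event spawns a particle effect, applies radial damage credited to the instigator's controller, fires a radial force impulse, then destroys the actor.
; BeginPlay is empty, and the one-second fuse and debug radius sphere are disconnected, so nothing in this graph triggers the explosion.
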(event EventBeginPlay)

(event EventExplode
  (bind _returnvalue (Transformation|GetActorLocation))
  (Effects|SpawnEmitteratLocation "/Game/Effects/P_Explosion_Small.P_Explosion_Small" _returnvalue)
  (Game|Damage|ApplyRadialDamage 1e+02 _returnvalue (Variables|Default|GetDamageRadius) 0 0 self (Game|GetInstigatorController) false "ECC_Visibility")
  (Class|RadialForceComponent|FireImpulse (Variables|Default|GetRadialForceComp))
  (Actor|DestroyActor))

(fn ConstructionScript)